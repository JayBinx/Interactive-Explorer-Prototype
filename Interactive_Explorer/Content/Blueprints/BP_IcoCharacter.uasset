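; Isometric player character that handles movement, interaction and elimination, and creates the HUD on BeginPlay.
; Enhanced Input movement offsets the control yaw by 45 degrees to match the isometric view.
; Interact runs a sphere trace at the character's location, sends an interact message to the single hit actor and broadcasts InteractableFound.
; Eliminate kills the health component, whose zero-durability event broadcasts Elimination and hides the cube mesh.
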(event `self.ReceiveBeginPlay`
  ;[1 1 1] Initialize UI
  (bind _returnvalue (`|CreateWidget` "/Game/UI/WBP_HUD.WBP_HUD_C" (`GameplayStatics.GetPlayerController` 0)))
  (`UserWidget.AddToViewport` _returnvalue 0))

(event `EnhancedInput|/Game/Input/Actions/IA_Move`
  (params (ActionValue :type "Vector2D Structure") (ElapsedSeconds :type "Float (double-precision)") (TriggeredSeconds :type "Float (double-precision)") (InputAction :type "InputAction Object Reference" :default "/Game/Input/Actions/IA_Move.IA_Move"))
  (bind (_returnvalue_roll _returnvalue_pitch _returnvalue_yaw) (`KismetMathLibrary.BreakRotator` (`self.GetControlRotation`)))
  (bind _returnvalue (+ _returnvalue_yaw 45.0))
  ;[1 1 1] Iscometric Character Movement
  (:`Triggered`
    (`self.AddMovementInput` (`KismetMathLibrary.GetRightVector` (`KismetMathLibrary.MakeRotator` 0.0 0.0 _returnvalue)) ActionValue_X)
    (`self.AddMovementInput` (`KismetMathLibrary.GetForwardVector` (`KismetMathLibrary.MakeRotator` 0.0 0.0 _returnvalue)) ActionValue_Y)))

(event `EnhancedInput|/Game/Input/Actions/IA_Interact`
  (params (ActionValue :type Boolean) (ElapsedSeconds :type "Float (double-precision)") (TriggeredSeconds :type "Float (double-precision)") (InputAction :type "InputAction Object Reference" :default "/Game/Input/Actions/IA_Interact.IA_Interact"))
  (bind _returnvalue (`self.K2_GetActorLocation`))
  ;[1 1 1] Interact w/ single object
  (:`Started`
    (bind _outhit (`KismetSystemLibrary.SphereTraceSingle` :`Start` _returnvalue :`End` _returnvalue :`Radius` (`self.Interact Radius`) :`TraceChannel` "TraceTypeQuery3" :`DrawDebugType` "ForDuration"))
    (bind (_bblockinghit _binitialoverlap _time _distance _location _impactpoint _normal _impactnormal _physmat _hitactor) (`GameplayStatics.BreakHitResult` _outhit))
    (message `/Game/Blueprints/BPI_Interactable.OnInteract` _hitactor self)
    (`self.Interactable Found` _hitactor)))

(event `/Game/Blueprints/BPI_Destructible.Eliminate`
  (params (EliminationCause :type "Actor Object Reference"))
  ;[1 1 1] Player Elimination
  (`/Game/Blueprints/BP_HealthComponent.Kill` (`self.BP_HealthComponent`)))

(event `self.BP_HealthComponent.Durabilty Zero`
  ;[1 1 1] Player Elimination
  (`self.Elimination` self)
  (`SceneComponent.SetVisibility` (`self.Cube`) false false))

(fn `UserConstructionScript`)