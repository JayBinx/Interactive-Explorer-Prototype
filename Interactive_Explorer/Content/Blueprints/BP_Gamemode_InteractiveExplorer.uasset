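; Game mode for the Interactive Explorer game that handles player death and the game over flow.
; On BeginPlay it finds the BP_IcoCharacter and binds to its elimination event.
; On death it spawns a scaled Niagara explosion, destroys the player after a short delay and calls game over.
; It then shows the game over widget with UI-only input and cursor, quitting the game when that widget's exit event fires.
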(event `self.ReceiveBeginPlay`
  (bind _returnvalue (`GameplayStatics.GetActorOfClass` "/Game/Blueprints/BP_IcoCharacter.BP_IcoCharacter_C"))
  (add `/Game/Blueprints/BP_IcoCharacter.Elimination` _returnvalue (delegate `Player Death`)))

(event `Player Death`
  (params (`Eliminated Object` :type "Actor Object Reference"))
  (bind _returnvalue (`GameplayStatics.GetPlayerController` 0))
  (`NiagaraFunctionLibrary.SpawnSystemAtLocation` "/Game/Effects/NPE_Explosion.NPE_Explosion" (`self.K2_GetActorLocation` `Eliminated Object`) (struct) (10.0 10.0 10.0))
  (`KismetSystemLibrary.Delay` 0.5)
  (`self.K2_DestroyActor` `Eliminated Object`)
  (`self.Game Over`)
  (bind _returnvalue_2 (`|CreateWidget` "/Game/UI/WBP_GameOverScreen.WBP_GameOverScreen_C"))
  (add `/Game/UI/WBP_GameOverScreen.ExitGame` _returnvalue_2 (delegate `End Game`))
  (`UserWidget.AddToViewport` _returnvalue_2 0)
  (`WidgetBlueprintLibrary.SetInputMode_UIOnlyEx` _returnvalue _returnvalue_2)
  (set `PlayerController.bShowMouseCursor` true _returnvalue))

(event `End Game`
  (`KismetSystemLibrary.QuitGame` null "Quit"))

(fn `UserConstructionScript`)